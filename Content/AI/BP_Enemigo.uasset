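; BP_Enemigo is an enemy character that chases the player and attacks with a sword slash montage.
; PawnSensing raises its speed and starts a single AI move toward the player, attacking on arrival.
; Damage plays a random hit montage, launches it along the player's forward vector and reduces health through BPCPlayerStats.
; When ReducirVida returns true, the mesh ragdolls and the health bar widget hides.
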(event OnSeePawn(PawnSensing)
  (params (Pawn :type Pawn%20Object%20Reference))
  (Variables|Default|SetIsSeeingPlayer? true)
  (Variables|/Script/Engine.CharacterMovementComponent|SetMaxWalkSpeed (Variables|Character|GetCharacterMovement) 7e+02)
  (CallFunction|FollowPlayer))

(event Custom|FollowPlayer
  (Variables|Default|SetcanAttack? true)
  (if (Variables|Default|GetIsSeeingPlayer?)
    (AI|AIMoveTo self "0, 0, 0" (Game|GetPlayerCharacter 0) 5.0 false
      (:OnSuccess
        (if (Variables|Default|GetcanAttack?)
          (Variables|Default|SetcanAttack? false)
          (Animation|Montage|PlayMontage (Variables|Character|GetMesh) "/Game/SwordAttack/MontageataqueSword/SwordAndShieldSlash2_UE_Montage.SwordAndShieldSlash2_UE_Montage"
            (:then
              (Utilities|FlowControl|Delay 0.5)
              (Variables|Default|SetcanAttack? true))))))
    (else
      (Variables|Default|SetIsSeeingPlayer? false))))

(event Game|Damage|EventAnyDamage
  (params (Damage :type Float%20%28single-precision%29) (DamageType :type Damage%20Type%20Object%20Reference) (InstigatedBy :type Controller%20Object%20Reference) (DamageCauser :type Actor%20Object%20Reference))
  (Animation|PlayAnimMontage (Utilities|Array|Get(acopy) (Variables|Default|GetHitAnims) (Math|Random|RandomIntegerinRange 0 (- (Utilities|Array|Length (Variables|Default|GetHitAnims)) 1))) 1.0 "None")
  (bind _asbp_third_person_character_2 (Utilities|Casting|CastToBP_ThirdPersonCharacter2 (Game|GetPlayerCharacter 0)))
  (Character|LaunchCharacter (* (Math|Vector|GetForwardVector (Transformation|GetActorRotation _asbp_third_person_character_2)) 4.5e+02) false false)
  (bind _jugador_muerto (Default|ReducirVida (Variables|Default|GetBPC_PlayerStats) Damage))
  (if _jugador_muerto
    (Physics|SetSimulatePhysics (Variables|Character|GetMesh) true)
    (Rendering|SetVisibility (Variables|Default|GetVida%20Widget) false false)))

(event EventTick
  (params (DeltaSeconds :type Float%20%28single-precision%29))
  (if (not (Variables|Default|GetIsSeeingPlayer?))
    (Components|Movement|StopMovementImmediately (Variables|Character|GetCharacterMovement))))

(event EventBeginPlay
  (bind _aswb_hud_enemigo (Utilities|Casting|CastToWB_HUD_ENEMIGO (UserInterface|GetWidget (Variables|Default|GetVida%20Widget))))
  (Variables|Default|SetBarraVida%20UI _aswb_hud_enemigo))

(fn ConstructionScript)
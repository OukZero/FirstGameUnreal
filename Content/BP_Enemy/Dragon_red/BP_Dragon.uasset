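; Dragon enemy that chases the player once pawn sensing spots them and bites on reaching them.
; AIMoveTo success plays the attack montage and damages Player-tagged actors in a sphere at the arrow, with a montage-length cooldown.
; Damage triggers a random hit montage, knockback along the player's forward and health reduction via BPCPlayerStats, ending in ragdoll.
; Tick halts movement until the player is seen and billboards the health widget to the camera.
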(event OnSeePawn(PawnSensing)
  (params (Pawn :type Pawn%20Object%20Reference))
  (Variables|Components|SetIsSeeingPlayer? true)
  (Variables|/Script/Engine.CharacterMovementComponent|SetMaxWalkSpeed (Variables|Character|GetCharacterMovement) 3.5e+02)
  (CallFunction|FollowPlayer))

(event Custom|Follow%20Player
  (Variables|Components|SetcanAttack? true)
  (if (Variables|Components|GetIsSeeingPlayer?)
    (AI|AIMoveTo self "0, 0, 0" (Game|GetPlayerCharacter 0) 5.0 false
      (:OnSuccess
        (if (Variables|Components|GetcanAttack?)
          (Variables|Components|SetcanAttack? false)
          (bind _returnvalue (Animation|PlayAnimMontage "/Game/FourEvilDragonsPBR/Animations/DragonTheUsurper/AttackMouthAnim_Montage.AttackMouthAnim_Montage" 1.0 "None"))
          (bind _outactors (Collision|SphereOverlapActors (Transformation|GetWorldLocation (Variables|Default|GetArrow1)) 1e+02 (Variables|Components|GetObject%20Types) 0))
          (bind _array_element (Utilities|Array|ForEachLoopwithBreak _outactors)
            (:LoopBody
              (if (Actor|ActorHasTag _array_element "Player")
                (Game|Damage|ApplyDamage _array_element 1e+01 0 0)))
            (:Completed
              (Utilities|FlowControl|Delay _returnvalue)
              (Variables|Components|SetcanAttack? true))))))
    (else
      (Variables|Components|SetIsSeeingPlayer? false))))

(event Game|Damage|EventAnyDamage
  (params (Damage :type Float%20%28single-precision%29) (DamageType :type Damage%20Type%20Object%20Reference) (InstigatedBy :type Controller%20Object%20Reference) (DamageCauser :type Actor%20Object%20Reference))
  (Animation|PlayAnimMontage (Utilities|Array|Get(acopy) (Variables|Components|GetHitAnims) (Math|Random|RandomIntegerinRange 0 (- (Utilities|Array|Length (Variables|Components|GetHitAnims)) 1))) 1.0 "None")
  (bind _asbp_third_person_character_2 (Utilities|Casting|CastToBP_ThirdPersonCharacter2 (Game|GetPlayerCharacter 0)))
  (Character|LaunchCharacter (* (Math|Vector|GetForwardVector (Transformation|GetActorRotation _asbp_third_person_character_2)) 4.5e+02) false false)
  (bind _jugador_muerto (Default|ReducirVida (Variables|Default|GetBPC_PlayerStats) Damage))
  (if _jugador_muerto
    (Physics|SetSimulatePhysics (Variables|Character|GetMesh) true)
    (Rendering|SetVisibility (Variables|Default|GetVida%20Widget) false false)))

(event EventTick
  (params (DeltaSeconds :type Float%20%28single-precision%29))
  (Utilities|FlowControl|Sequence
    (:then_0
      (if (not (Variables|Components|GetIsSeeingPlayer?))
        (Components|Movement|StopMovementImmediately (Variables|Character|GetCharacterMovement))))
    (:then_1
      (Transformation|SetWorldRotation (Variables|Default|GetVida%20Widget) (Math|Rotator|FindLookatRotation (Transformation|GetWorldLocation (Variables|Default|GetVida%20Widget)) (Transformation|GetWorldLocation (Variables|/Script/Engine.PlayerCameraManager|GetTransformComponent (Game|GetPlayerCameraManager 0)))) false false))))

(event EventBeginPlay
  (bind _aswb_hud_enemigo (Utilities|Casting|CastToWB_HUD_ENEMIGO (UserInterface|GetWidget (Variables|Default|GetVida%20Widget))))
  (Variables|Components|SetBarraVida%20UI _aswb_hud_enemigo))

(fn ConstructionScript)